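; BP_TPSPlayer is a third-person shooter player Blueprint whose graph logic is entirely disconnected, so none of it runs.
; The leftover nodes switch between grenade and sniper guns, create crosshair and scope widgets, and zoom the sniper by changing camera FOV.
; Other remnants cover crouching, restarting a fire camera shake, and a camera line trace that spawns explosions and pushes physics objects.
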(event `InputAction|Fire`
  (params (Key :type "Key Structure")))

(event `self.ReceiveBeginPlay`
  ;[1 1 1] 시작할 때 1번 총 선택
)

(event `InputAction|GrenadeGun` :overrideparent false
  (params (Key :type "Key Structure"))
  ;[1 1 1] 1번을 누르면 Grenade Gun으로 변경
)

(event `InputAction|Zoom` :overrideparent false
  (params (Key :type "Key Structure"))
  ;[1 1 1] Sniper Zoom
)

(event `InputAction|SniperGun` :overrideparent false
  (params (Key :type "Key Structure"))
  ;[1 1 1] 2번을 누르면 Sniper Gun으로 변경
)

(event `ChangeGrenadeGun`
  (params (bShowGrenade :type Boolean))
  ;[1 1 1] Grenade Gun으로 변경
)

(event `InputAction|Crouch` :overrideparent false
  (params (Key :type "Key Structure"))
  ;[1 1 1] Action Crouch
)

(fn `UserConstructionScript`)