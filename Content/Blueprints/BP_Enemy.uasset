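; Enemy character Blueprint with an overhead HP widget and a damage reaction animation.
; BeginPlay hands itself to the WB_EnemyHP widget as owner, and Tick turns that widget toward the player camera, keeping it upright along the actor's up axis.
; OnMyDamage plays the enemy montage from the given section name.
; An Idle/Move/Attack chase state machine remains in the graph but is disconnected and never runs.
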(event `self.ReceiveTick`
  (params (DeltaSeconds :type "Float (single-precision)"))
  (`SceneComponent.K2_SetWorldRotation` (`self.WidgetHP`) (`KismetMathLibrary.MakeRotFromXZ` (- (`self.K2_GetActorLocation` (`GameplayStatics.GetPlayerCameraManager` 0)) (`self.K2_GetActorLocation`)) (`self.GetActorUpVector`)) false false))

(event `self.ReceiveBeginPlay`
  (bind _aswb_enemy_hp (cast `/Game/UI/WB_EnemyHP` (`WidgetComponent.GetWidget` (`self.WidgetHP`))))
  (set `/Game/UI/WB_EnemyHP.owner` self _aswb_enemy_hp))

(event `self.OnMyDamage`
  (params (SectionName :type Name))
  (`self.PlayAnimMontage` "/Game/Blueprints/EnemyAnimMontage.EnemyAnimMontage" 1.0 SectionName))

(fn `UserConstructionScript`)